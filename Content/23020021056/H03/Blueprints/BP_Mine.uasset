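; BP_Mine is a re-armable mine that launches an overlapping Character straight upward.
; On overlap, a DoOnce gate hides the mine mesh and applies the launch, so it fires only once until reset.
; The actor enables input from player 0 on BeginPlay, so pressing R shows the mesh again, prints a Turkish re-armed message and resets the gate.
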(event `self.ReceiveBeginPlay`
  (`self.EnableInput` (`GameplayStatics.GetPlayerController` 0)))

(event `self.ReceiveActorBeginOverlap`
  (params (OtherActor :type "Actor Object Reference"))
  (bind _ascharacter (cast `Character` OtherActor))
  (`/Engine/EditorBlueprintResources/StandardMacros.DoOnce` false :!label _label
    (:`Completed`
      (`SceneComponent.SetVisibility` (`self.MineMesh`) false false)
      (`Character.LaunchCharacter` _ascharacter (`KismetMathLibrary.MakeVector` 0.0 0.0 1200.0) false false))))

(event `Key|R`
  (params (Key :type "Key Structure"))
  (:`Pressed`
    (`SceneComponent.SetVisibility` (`self.MineMesh`) true false)
    (`KismetSystemLibrary.PrintString` "Mayın yeniden kuruldu.")
    (goto _label :!via `Reset`)))

(fn `UserConstructionScript`)