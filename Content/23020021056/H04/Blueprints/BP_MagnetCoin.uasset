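; BP_MagnetCoin is a spinning coin pickup that flies toward the player when they come within PullRadius.
; Tick rotates the coin in yaw and, within that radius, moves it straight at player character 0 at Speed, scaled by delta time and without sweep.
; Overlap with any Character prints a Turkish "coin collected" message and destroys the coin, with no score or inventory update.
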(event `self.ReceiveTick`
  (params (DeltaSeconds :type "Float (single-precision)"))
  (bind _returnvalue (`GameplayStatics.GetPlayerCharacter` 0))
  (bind _returnvalue_2 (`self.K2_GetActorLocation`))
  (`self.K2_AddActorLocalRotation` (`KismetMathLibrary.MakeRotator` 0.0 0.0 (* DeltaSeconds 180.0)))
  (if (< (`self.GetDistanceTo` _returnvalue) (`self.PullRadius`))
    (`self.K2_SetActorLocation` (+ _returnvalue_2 (* (`KismetMathLibrary.GetDirectionUnitVector` _returnvalue_2 (`self.K2_GetActorLocation` _returnvalue)) (* (`self.Speed`) DeltaSeconds))))))

(event `self.ReceiveActorBeginOverlap`
  (params (OtherActor :type "Actor Object Reference"))
  (cast `Character` OtherActor)
  (`KismetSystemLibrary.PrintString` "Coin Toplandı!")
  (`self.K2_DestroyActor`))

(fn `UserConstructionScript`)