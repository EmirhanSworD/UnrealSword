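; Loot chest actor that rolls a random item, rarity and power when the player presses E nearby, up to ten times.
; A seeded random stream drives the rolls, making loot sequences reproducible.
; A math expression computes power from base power, a rarity bonus and a roll bounded by chest level.
; Each opening tints the chest's dynamic material from grey toward gold by power and prints the result.
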(event EventBeginPlay
  (Math|Random|SetRandomStreamSeed (Variables|Default|GetStream) (Variables|Default|GetSeed))
  (bind _returnvalue (Rendering|Material|CreateDynamicMaterialInstance (Variables|Default|GetChestBody) 0 "/Game/23020021056/H03/Materials/M_FlowBase.M_FlowBase" "None" :!class /Script/Engine.PrimitiveComponent))
  (Variables|Default|SetDynMat _returnvalue)
  (Input|EnableInput (Game|GetPlayerController 0)))

(event Input|KeyboardEvents|E
  (params (Key :type Key%20Structure))
  (:Pressed
    (if (< (Transformation|GetDistanceTo (Game|GetPlayerCharacter 0)) 3e+02)
      (Utilities|FlowControl|DoN 10
        (:Exit
          (CallFunction|OpenChest))))))

(fn ConstructionScript)

(fn RarityBonus
  (switch Utilities|FlowControl|Switch|SwitchonE_Rarity (Variables|Default|GetRarity)
    (:NewEnumerator0
      (return 0.0))
    (:NewEnumerator1
      (return 0.5))
    (:NewEnumerator2
      (return 1.5))))

(fn RollRarity
  (LocalVariables|SetR (Math|Random|RandomFloatfromStream (Variables|Default|GetStream)))
  (if (< (LocalVariables|GetR) 0.6)
    (Variables|Default|SetRarity "NewEnumerator0")
    (elif (< (LocalVariables|GetR) 0.9)
      (Variables|Default|SetRarity "NewEnumerator1")
      (else
        (Variables|Default|SetRarity "NewEnumerator2")))))

(fn CalculatePower
  (params (Base :type Float%20%28double-precision%29) (RarityBonus :type Float%20%28double-precision%29) (Roll :type Float%20%28double-precision%29))
  (return (|((Base*(1+RarityBonus))+Roll) Base RarityBonus Roll)))

(fn OpenChest
  (CallFunction|RollRarity)
  (bind _bonus (CallFunction|RarityBonus))
  (bind _power (CallFunction|CalculatePower (Variables|Default|GetBasePower) _bonus (Math|Conversions|ToFloat(Integer) (Math|Random|RandomIntegerinRangefromStream (Variables|Default|GetStream) 0 (Variables|Default|GetChestLevel)))))
  (Variables|Default|SetPower _power)
  (Rendering|Material|SetVectorParameterValue (Variables|Default|GetDynMat) "Color" (Math|Color|Lerp(LinearColor) "(R=0.200000,G=0.200000,B=0.200000,A=1.000000)" "(R=1.000000,G=0.750000,B=0.100000,A=1.000000)" (Math|Float|MapRangeClamped (Variables|Default|GetPower) 1e+01 4e+01 0.0 1.0)) :!class /Script/Engine.MaterialInstanceDynamic)
  (Development|PrintText (Utilities|Text|FormatText "{Esya} ({Nadirlik}) Guc: {Guc}" (.OutItem (Utilities|Array|RandomFromStream (Variables|Default|GetItems) (Variables|Default|GetStream))) (Utilities|String|EnumtoString (Variables|Default|GetRarity)) (Variables|Default|GetPower))))