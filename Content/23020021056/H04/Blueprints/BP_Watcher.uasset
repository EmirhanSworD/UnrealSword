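; BP_Watcher is a sentry actor that shows when the player enters its view cone.
; Each Tick it draws a debug cone at a raised origin and calls CanSeePlayer, which combines a ViewDistance check with a forward-vector dot product against ConeDot, without an occlusion trace.
; On detection it switches Body to the alert material and prints a Turkish "seen" message; otherwise it applies the calm material.
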(event `self.ReceiveTick`
  (params (DeltaSeconds :type "Float (single-precision)"))
  (`KismetSystemLibrary.DrawDebugConeInDegrees` (+ (`self.K2_GetActorLocation`) (`KismetMathLibrary.MakeVector` 0.0 0.0 185.0)) (`self.GetActorForwardVector`) (`self.ViewDistance`) 45.0 45.0 24 (struct :`R` 1.0 :`G` 0.75 :`B` 0.1 :`A` 1.0) 0.0 1.0)
  (bind _seen (`self.CanSeePlayer`))
  (if _seen
    (`PrimitiveComponent.SetMaterial` (`self.Body`) 0 "/Game/23020021056/H04/Materials/MI_WatcherAlert.MI_WatcherAlert")
    (`KismetSystemLibrary.PrintString` "GÖRÜLDÜN!" true true (struct :`G` 0.66 :`B` 1.0 :`A` 1.0) 2.0 "Gozcu")
    (else
      (`PrimitiveComponent.SetMaterial` (`self.Body`) 0 "/Game/23020021056/H04/Materials/MI_WatcherCalm.MI_WatcherCalm"))))

(fn `CanSeePlayer`
  (returns (Seen :type Boolean))
  (bind _returnvalue (`GameplayStatics.GetPlayerCharacter` 0))
  (bind _returnvalue_2 (`KismetMathLibrary.Dot_VectorVector` (`self.GetActorForwardVector`) (`KismetMathLibrary.GetDirectionUnitVector` (`self.K2_GetActorLocation`) (`self.K2_GetActorLocation` _returnvalue))))
  (set `self.DotValue` _returnvalue_2)
  (return (and (< (`self.GetDistanceTo` _returnvalue) (`self.ViewDistance`)) (> _returnvalue_2 (`self.ConeDot`)))))

(fn `UserConstructionScript`)