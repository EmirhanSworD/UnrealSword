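; Grid manager for a timed match-3 puzzle that spawns BP_VizePuzzleBlock actors and drives the score, timer and status HUD.
; Three selected blocks of one type in a straight line break, with bombs chain-detonating their 3x3 neighbors.
; Columns then collapse and refill, and rescans trigger cascades with multiplied points.
; Looping timers count down to game over and reshuffle inactive block types, pausing the shuffle while matches resolve.
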(event `self.ReceiveBeginPlay`
  (bind _returnvalue (`|CreateWidget` "/Game/23020021056/H05/UI/W_VizeHUD.W_VizeHUD_C" (`GameplayStatics.GetPlayerController` 0)))
  (set `self.VizeHud` _returnvalue)
  (`UserWidget.AddToViewport` _returnvalue 0)
  (`self.CreateGrid` self)
  (bind _returnvalue_2 (`KismetSystemLibrary.K2_SetTimer` self "RandomizeBlocks" 2.5 true))
  (set `self.RandomizeTimer` _returnvalue_2)
  (bind _returnvalue_3 (`KismetSystemLibrary.K2_SetTimer` self "CountdownTick" 1.0 true))
  (set `self.CountdownTimer` _returnvalue_3)
  (`self.UpdateHud` self))

(event `RandomizeBlocks`
  (for _array_element (`self.VizeBlocks`)
    (`/Engine/EditorBlueprintResources/StandardMacros.IsValid` _array_element
      (:`Is Valid`
        (if (not (`/Game/23020021056/H05/Blueprints/BP_VizePuzzleBlock.bIsActive` _array_element))
          (`/Game/23020021056/H05/Blueprints/BP_VizePuzzleBlock.AssignBlockType` _array_element (`KismetMathLibrary.RandomIntegerInRange` 0 2)))))))

(event `CheckMatch`
  (bind _activeblocks (`self.ActiveBlocks`))
  (bind _output (`|GetArrayItem` _activeblocks))
  (bind _output_2 (`|GetArrayItem` _activeblocks 1))
  (bind _output_3 (`|GetArrayItem` _activeblocks 2))
  (bind _same (`self.AreSameType` self _output _output_2 _output_3))
  (bind _inline (`self.AreInLine` self _output _output_2 _output_3))
  (if (and _same _inline)
    (`self.BreakMatched` self)
    (else
      (`self.ResetSelection` self))))

(event `CheckCascadeMatches`
  (bind _size (`self.Size`))
  (if (`self.bGameOver`)
    (set `self.bBreaking` false)
    (else
      (`KismetArrayLibrary.Array_Clear` (`self.ActiveBlocks`))
      (for _index (range (+ (- _size 1) 1))
        (for _index_2 (range (+ (- (- _size 2) 1) 1))
          (bind _returnvalue (+ (* _index _size) _index_2))
          (bind _returnvalue_2 (+ _returnvalue 1))
          (bind _returnvalue_3 (+ _returnvalue 2))
          (bind _same (`self.AreSameType` self _returnvalue _returnvalue_2 _returnvalue_3))
          (if _same
            (`KismetArrayLibrary.Array_AddUnique` (`self.ActiveBlocks`) _returnvalue)
            (`KismetArrayLibrary.Array_AddUnique` (`self.ActiveBlocks`) _returnvalue_2)
            (`KismetArrayLibrary.Array_AddUnique` (`self.ActiveBlocks`) _returnvalue_3))))
      (for _index_3 (range (+ (- (- _size 2) 1) 1))
        (for _index_4 (range (+ (- _size 1) 1))
          (bind _returnvalue_4 (+ (* _index_3 _size) _index_4))
          (bind _returnvalue_5 (+ (* (+ _index_3 1) _size) _index_4))
          (bind _returnvalue_6 (+ (* (+ _index_3 2) _size) _index_4))
          (bind _same_2 (`self.AreSameType` self _returnvalue_4 _returnvalue_5 _returnvalue_6))
          (if _same_2
            (`KismetArrayLibrary.Array_AddUnique` (`self.ActiveBlocks`) _returnvalue_4)
            (`KismetArrayLibrary.Array_AddUnique` (`self.ActiveBlocks`) _returnvalue_5)
            (`KismetArrayLibrary.Array_AddUnique` (`self.ActiveBlocks`) _returnvalue_6))))
      (if (> (`KismetArrayLibrary.Array_Length` (`self.ActiveBlocks`)) 0)
        (set `self.CascadeCount` (+ (`self.CascadeCount`) 1))
        (`self.BreakMatched` self)
        (else
          (set `self.CascadeCount` 0)
          (set `self.bBreaking` false)
          (`KismetSystemLibrary.K2_UnPauseTimerHandle` (`self.RandomizeTimer`)))))))

(event `BreakMatched`
  (set `self.bBreaking` true)
  (`KismetSystemLibrary.K2_PauseTimerHandle` (`self.RandomizeTimer`))
  (`self.ExpandBombs` self)
  (set `self.TempPoints` (+ (* (* (`KismetArrayLibrary.Array_Length` (`self.ActiveBlocks`)) 10) (`self.CascadeCount`)) (* (`self.TempBombsHit`) 50)))
  (set `self.Score` (+ (`self.Score`) (`self.TempPoints`)))
  (if (> (`self.TempBombsHit`) 0)
    (set `self.StatusMessage` (`KismetStringLibrary.Concat_StrStr` "BOMBA PATLADI! +" (`KismetStringLibrary.Conv_IntToString` (`self.TempPoints`))))
    (elif (> (`self.CascadeCount`) 1)
      (set `self.StatusMessage` (`KismetStringLibrary.Concat_StrStr` (`KismetStringLibrary.Concat_StrStr` "ZINCIR x" (`KismetStringLibrary.Conv_IntToString` (`self.CascadeCount`))) (`KismetStringLibrary.Concat_StrStr` "! +" (`KismetStringLibrary.Conv_IntToString` (`self.TempPoints`)))))
      (else
        (set `self.StatusMessage` (`KismetStringLibrary.Concat_StrStr` "Eslesme! +" (`KismetStringLibrary.Conv_IntToString` (`self.TempPoints`)))))))
  (`self.UpdateHud` self)
  (for _array_element (`self.ActiveBlocks`)
    (set `self.TempBlock` (`|GetArrayItem` (`self.VizeBlocks`) _array_element))
    (`KismetArrayLibrary.Array_Set` (`self.VizeBlocks`) _array_element (`self.NullBlock`) true)
    (`/Engine/EditorBlueprintResources/StandardMacros.IsValid` (`self.TempBlock`)
      (:`Is Valid`
        (`/Game/23020021056/H05/Blueprints/BP_VizePuzzleBlock.BreakBlock` (`self.TempBlock`)))))
  (`KismetArrayLibrary.Array_Clear` (`self.ActiveBlocks`))
  (`KismetSystemLibrary.Delay` 0.5)
  (`self.ApplyGravityAndRefill` self)
  (`KismetSystemLibrary.Delay` 0.45)
  (`self.CheckCascadeMatches` self))

(event `CountdownTick`
  (set `self.TimeLeft` (- (`self.TimeLeft`) 1))
  (`self.UpdateHud` self)
  (if (<= (`self.TimeLeft`) 0)
    (`self.EndGame` self)))

(fn `ApplyGravityAndRefill`
  (bind _tempwriterow (`self.TempWriteRow`))
  (bind _size (`self.Size`))
  (bind _spacing (`self.Spacing`))
  (for _index (range (+ (- _size 1) 1))
    (set `self.TempWriteRow` 0)
    (for _index_2 (range (+ (- _size 1) 1))
      (bind _returnvalue (+ (* _index_2 _size) _index))
      (set `self.TempBlock` (`|GetArrayItem` (`self.VizeBlocks`) _returnvalue))
      (`/Engine/EditorBlueprintResources/StandardMacros.IsValid` (`self.TempBlock`)
        (:`Is Valid`
          (if (!= _index_2 _tempwriterow)
            (bind _returnvalue_2 (+ (* _tempwriterow _size) _index))
            (`KismetArrayLibrary.Array_Set` (`self.VizeBlocks`) _returnvalue_2 (`self.TempBlock`) true)
            (`KismetArrayLibrary.Array_Set` (`self.VizeBlocks`) _returnvalue (`self.NullBlock`) true)
            (set `/Game/23020021056/H05/Blueprints/BP_VizePuzzleBlock.GridIndex` _returnvalue_2 (`self.TempBlock`))
            (`/Game/23020021056/H05/Blueprints/BP_VizePuzzleBlock.StartFallTo` (`self.TempBlock`) (+ (`self.K2_GetActorLocation`) (`KismetMathLibrary.MakeVector` (* _tempwriterow _spacing) (* _index _spacing)))))
          (set `self.TempWriteRow` (+ _tempwriterow 1)))))
    (while (< (`self.TempWriteRow`) _size)
      (`self.CreateVizeBlock` self (`self.TempWriteRow`) _index true)
      (set `self.TempWriteRow` (+ (`self.TempWriteRow`) 1)))))

(fn `AreInLine`
  (params (A :type Integer) (B :type Integer) (C :type Integer))
  (returns (InLine :type Boolean))
  (bind _size (`self.Size`))
  (bind _returnvalue (mod B _size))
  (bind _returnvalue_2 (/ B _size))
  (bind _returnvalue_3 (- (`KismetMathLibrary.Max` (`KismetMathLibrary.Max` A B) C) (`KismetMathLibrary.Min` (`KismetMathLibrary.Min` A B) C)))
  (return (or (and (and (== (/ A _size) _returnvalue_2) (== _returnvalue_2 (/ C _size))) (== _returnvalue_3 2)) (and (and (== (mod A _size) _returnvalue) (== _returnvalue (mod C _size))) (== _returnvalue_3 (* 2 _size))))))

(fn `AreSameType`
  (params (A :type Integer) (B :type Integer) (C :type Integer))
  (returns (Same :type Boolean))
  (bind _vizeblocks (`self.VizeBlocks`))
  (bind _output (`|GetArrayItem` _vizeblocks A))
  (bind _output_2 (`|GetArrayItem` _vizeblocks B))
  (bind _output_3 (`|GetArrayItem` _vizeblocks C))
  (bind _blocktype (`/Game/23020021056/H05/Blueprints/BP_VizePuzzleBlock.BlockType` _output_2))
  (`/Engine/EditorBlueprintResources/StandardMacros.IsValid` _output
    (:`Is Valid`
      (`/Engine/EditorBlueprintResources/StandardMacros.IsValid` _output_2
        (:`Is Valid`
          (`/Engine/EditorBlueprintResources/StandardMacros.IsValid` _output_3
            (:`Is Valid`
              (return (and (== (`/Game/23020021056/H05/Blueprints/BP_VizePuzzleBlock.BlockType` _output) _blocktype) (== _blocktype (`/Game/23020021056/H05/Blueprints/BP_VizePuzzleBlock.BlockType` _output_3)))))
            (:`Is Not Valid`
              (return false))))
        (:`Is Not Valid`
          (return false))))
    (:`Is Not Valid`
      (return false))))

(fn `ClearSelection`
  (`self.ResetSelection` self))

(fn `CreateGrid`
  (bind _size (`self.Size`))
  (bind _output (`|GetArrayItem` (`self.VizeBlocks`) 5))
  (for _index (range (+ (- _size 1) 1))
    (for _index_2 (range (+ (- _size 1) 1))
      (`self.CreateVizeBlock` self _index _index_2 false)))
  (`/Engine/EditorBlueprintResources/StandardMacros.IsValid` _output
    (:`Is Valid`
      (`/Game/23020021056/H05/Blueprints/BP_VizePuzzleBlock.MakeBomb` _output))))

(fn `CreateVizeBlock`
  (params (Row :type Integer) (Col :type Integer) (StartAbove :type Boolean))
  (returns (NewBlock :type "/Game/23020021056/H05/Blueprints/BP_VizePuzzleBlock Object Reference"))
  (bind _returnvalue (`self.K2_GetActorLocation`))
  (bind _size (`self.Size`))
  (bind _spacing (`self.Spacing`))
  (bind _returnvalue_2 (+ (* Row _size) Col))
  (bind _returnvalue_3 (`|SpawnActorFromClass` "/Game/23020021056/H05/Blueprints/BP_VizePuzzleBlock.BP_VizePuzzleBlock_C" (`KismetMathLibrary.MakeTransform` (+ _returnvalue (`KismetMathLibrary.MakeVector` (* (select `bool` StartAbove :`false` Row :`true` (+ _size 1)) _spacing) (* Col _spacing)))) "AlwaysSpawn" "MultiplyWithRoot" null 0 null null))
  (`/Game/23020021056/H05/Blueprints/BP_VizePuzzleBlock.InitBlock` _returnvalue_3 self _returnvalue_2 (`KismetMathLibrary.RandomIntegerInRange` 0 2) (< (`KismetMathLibrary.RandomIntegerInRange` 0 99) (`self.BombChancePercent`)) (+ _returnvalue (`KismetMathLibrary.MakeVector` (* Row _spacing) (* Col _spacing))))
  (`KismetArrayLibrary.Array_Set` (`self.VizeBlocks`) _returnvalue_2 _returnvalue_3 true)
  (return _returnvalue_3))

(fn `EndGame`
  (bind _vizehud (`self.VizeHud`))
  (set `self.bGameOver` true)
  (`KismetSystemLibrary.K2_ClearAndInvalidateTimerHandle` (`self.RandomizeTimer`))
  (`KismetSystemLibrary.K2_ClearAndInvalidateTimerHandle` (`self.CountdownTimer`))
  (set `self.StatusMessage` (`KismetStringLibrary.Concat_StrStr` "OYUN BITTI! Toplam Puan: " (`KismetStringLibrary.Conv_IntToString` (`self.Score`))))
  (`self.UpdateHud` self)
  (`KismetSystemLibrary.PrintString` "OYUN BITTI")
  (`/Engine/EditorBlueprintResources/StandardMacros.IsValid` _vizehud
    (:`Is Valid`
      (`Widget.SetVisibility` (`/Game/23020021056/H05/UI/W_VizeHUD.txtGameOver` _vizehud) "Visible"))))

(fn `ExpandBombs`
  (returns (BombsTriggered :type Integer))
  (bind _size (`self.Size`))
  (set `self.TempBombsHit` 0)
  (set `self.FoundBomb` true)
  (while (`self.FoundBomb`)
    (set `self.FoundBomb` false)
    (for _index (range (+ (- (`KismetArrayLibrary.Array_Length` (`self.ActiveBlocks`)) 1) 1))
      (bind _output (`|GetArrayItem` (`self.ActiveBlocks`) _index))
      (set `self.TempBlock` (`|GetArrayItem` (`self.VizeBlocks`) _output))
      (`/Engine/EditorBlueprintResources/StandardMacros.IsValid` (`self.TempBlock`)
        (:`Is Valid`
          (if (and (`/Game/23020021056/H05/Blueprints/BP_VizePuzzleBlock.IsBomb` (`self.TempBlock`)) (not (`/Game/23020021056/H05/Blueprints/BP_VizePuzzleBlock.BombDetonated` (`self.TempBlock`))))
            (set `/Game/23020021056/H05/Blueprints/BP_VizePuzzleBlock.BombDetonated` true (`self.TempBlock`))
            (set `self.TempBombsHit` (+ (`self.TempBombsHit`) 1))
            (set `self.FoundBomb` true)
            (for _index_2 (range 3)
              (for _index_3 (range 3)
                (bind _returnvalue (+ (/ _output _size) (- _index_2 1)))
                (bind _returnvalue_2 (+ (mod _output _size) (- _index_3 1)))
                (if (and (and (>= _returnvalue 0) (< _returnvalue _size)) (and (>= _returnvalue_2 0) (< _returnvalue_2 _size)))
                  (`KismetArrayLibrary.Array_AddUnique` (`self.ActiveBlocks`) (+ (* _returnvalue _size) _returnvalue_2))))))))))
  (return (`self.TempBombsHit`)))

(fn `ResetSelection`
  (for _array_element (`self.ActiveBlocks`)
    (set `self.TempBlock` (`|GetArrayItem` (`self.VizeBlocks`) _array_element))
    (`/Engine/EditorBlueprintResources/StandardMacros.IsValid` (`self.TempBlock`)
      (:`Is Valid`
        (`/Game/23020021056/H05/Blueprints/BP_VizePuzzleBlock.MakeSelectable` (`self.TempBlock`)))))
  (`KismetArrayLibrary.Array_Clear` (`self.ActiveBlocks`)))

(fn `UpdateHud`
  (bind _vizehud (`self.VizeHud`))
  (`/Engine/EditorBlueprintResources/StandardMacros.IsValid` _vizehud
    (:`Is Valid`
      (`TextBlock.SetText` (`/Game/23020021056/H05/UI/W_VizeHUD.txtScore` _vizehud) (`KismetTextLibrary.Conv_StringToText` (`KismetStringLibrary.Concat_StrStr` "Puan: " (`KismetStringLibrary.Conv_IntToString` (`self.Score`)))))
      (`TextBlock.SetText` (`/Game/23020021056/H05/UI/W_VizeHUD.txtTime` _vizehud) (`KismetTextLibrary.Conv_StringToText` (`KismetStringLibrary.Concat_StrStr` "Sure: " (`KismetStringLibrary.Conv_IntToString` (`self.TimeLeft`)))))
      (`TextBlock.SetText` (`/Game/23020021056/H05/UI/W_VizeHUD.txtStatus` _vizehud) (`KismetTextLibrary.Conv_StringToText` (`self.StatusMessage`))))))

(fn `UserConstructionScript`)

(fn `VizeBlockSelected`
  (params (Block :type "/Game/23020021056/H05/Blueprints/BP_VizePuzzleBlock Object Reference"))
  (if (or (`self.bGameOver`) (`self.bBreaking`))
    (`/Game/23020021056/H05/Blueprints/BP_VizePuzzleBlock.MakeSelectable` Block)
    (else
      (`KismetArrayLibrary.Array_AddUnique` (`self.ActiveBlocks`) (`/Game/23020021056/H05/Blueprints/BP_VizePuzzleBlock.GridIndex` Block))
      (if (== (`KismetArrayLibrary.Array_Length` (`self.ActiveBlocks`)) 3)
        (set `self.CascadeCount` 1)
        (`self.CheckMatch` self)))))