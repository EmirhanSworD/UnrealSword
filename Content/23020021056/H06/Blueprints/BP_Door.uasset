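; BP_Door is a door that opens only while every pressure plate in its Plates array is pressed.
; On BeginPlay it binds to each plate's pressed and released events and keeps a running count of pressed plates.
; When the count matches the array length, the door mesh slides up over one second and the OnOpened dispatcher fires.
; Releasing any plate while open slides it back down.
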(event `self.ReceiveBeginPlay`
  (for _array_element (`self.Plates`)
    (add `/Game/23020021056/H06/Blueprints/BP_PressurePlate.OnPlatePressed` _array_element (delegate `PlatePressed`))
    (add `/Game/23020021056/H06/Blueprints/BP_PressurePlate.OnPlateReleased` _array_element (delegate `PlateReleased`))))

(event `PlatePressed`
  (set `self.PressedCount` (+ (`self.PressedCount`) 1))
  (if (== (`self.PressedCount`) (`KismetArrayLibrary.Array_Length` (`self.Plates`)))
    (`self.OpenDoor`)))

(event `PlateReleased`
  (set `self.PressedCount` (- (`self.PressedCount`) 1))
  (if (`self.bOpen`)
    (`self.CloseDoor`)))

(event `OpenDoor`
  (set `self.bOpen` true)
  (`KismetSystemLibrary.MoveComponentTo` (`self.DoorMesh`) (`KismetMathLibrary.MakeVector` 0.0 0.0 460.0) (struct) false false 1.0)
  (`self.OnOpened` self))

(event `CloseDoor`
  (set `self.bOpen` false)
  (`KismetSystemLibrary.MoveComponentTo` (`self.DoorMesh`) (`KismetMathLibrary.MakeVector` 0.0 0.0 150.0) (struct) false false 1.0))

(fn `UserConstructionScript`)